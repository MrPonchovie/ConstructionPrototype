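; Medical syringe weapon (HD item) that revives downed characters.
; Firing, on the cosmetic-capable side, waits a retriggerable fire delay, then traces for a pawn from the muzzle along the first-person camera's forward vector if still equipped.
; A revivable hit goes to ServerReviveCharacter with the target's right clavicle socket location.
; That event rechecks eligibility, has the target's revive component revive it there and consumes one ammo.
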(event `ServerReviveCharacter`
  (params (Target :type "Actor Object Reference") (ReviveLocation :type "Vector Structure"))
  (bind (_isrevivable _revivecomponent) (`self.CheckIfRevivable` Target))
  (if _isrevivable
    (`/ConstructionPrototype/Medical/Components/AC_HDReviveCharacter.ReviveCharacterAtLocation` _revivecomponent ReviveLocation)
    (`DFBaseAmmoClip.ConsumeAmmo` (`self.CurrentAmmoClip`) 1)))

(event `self.ReceiveOnLeaveInventory`
  (params (LastOwner :type "DFBaseCharacter Object Reference"))
  (`parent.ReceiveOnLeaveInventory` LastOwner))

(event `self.ReceiveOnEnterInventory`
  (params (NewOwner :type "DFBaseCharacter Object Reference") (LastOwner :type "DFBaseCharacter Object Reference"))
  (`parent.ReceiveOnEnterInventory` NewOwner LastOwner))

(event `self.ReceiveOnEquip`
  (params (LastItem :type "DFBaseItem Object Reference"))
  (`parent.ReceiveOnEquip` LastItem))

(event `self.ReceiveFire`
  (`/Engine/EditorBlueprintResources/StandardMacros.Can Execute Cosmetic Events`
    (:`True`
      (`KismetSystemLibrary.RetriggerableDelay` (`self.FireDelay`))
      (if (`self.IsEquipped`)
        (bind _asbp_hdplayer_character_base (cast `/HDCore/Core/BP_HDPlayerCharacterBase` (`self.GetPawnOwner`)))
        (bind _hitactor (`self.TraceForPawn` (`SceneComponent.K2_GetComponentLocation` (`self.Muzzle`)) (`SceneComponent.GetForwardVector` (`DFBasePlayerCharacter.GetCamera1P` _asbp_hdplayer_character_base))))
        (bind (_isrevivable _revivecomponent) (`self.CheckIfRevivable` _hitactor))
        (if _isrevivable
          (`self.ServerReviveCharacter` _hitactor (`SceneComponent.GetSocketLocation` (`Character.Mesh` (`/ConstructionPrototype/Medical/Components/AC_HDReviveCharacter.GetOwningPawn` _revivecomponent)) "clavicle_r")))))))

(fn `UserConstructionScript`
  (`parent.UserConstructionScript`))