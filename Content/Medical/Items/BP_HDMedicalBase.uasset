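; Base Blueprint for medical items that gates firing on whether the player is aiming at a pawn they can revive.
; CheckToHeal line-traces from the first-person camera within heal range, then queries the hit actor's revive component through IF_Revivable using the owner's team.
; The resulting CanHeal flag combines with the parent's CanFire.
; Both fire events are empty here, and CheckToHeal has no caller in this Blueprint.
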(event `PrimaryFire`)

(event `AltFire`)

(event `self.ReceiveBeginPlay`
  (`parent.ReceiveBeginPlay`)
  (`/Engine/EditorBlueprintResources/StandardMacros.Can Execute Cosmetic Events`
    (:`True`
      (set `self.CanHeal` false))))

(fn `CanFire`
  (returns (ReturnValue :type Boolean))
  (return (and (`self.CanHeal`) (`parent.CanFire`))))

(fn `CheckIfRevivable`
  (params (TestObject :type "Object Object Reference"))
  (returns (IsRevivable :type Boolean) (ReviveComponent :type "/ConstructionPrototype/Medical/Components/AC_HDReviveCharacter Object Reference"))
  (bind _returnvalue (`KismetSystemLibrary.DoesImplementInterface` TestObject "/ConstructionPrototype/Medical/Interfaces/IF_Revivable.IF_Revivable_C"))
  (if _returnvalue
    (bind _revivecomponent (message `/ConstructionPrototype/Medical/Interfaces/IF_Revivable.GetReviveComponent` TestObject))
    (return (`/ConstructionPrototype/Medical/Components/AC_HDReviveCharacter.IsRevivable` _revivecomponent (`DFBlueprintFunctions.GetTeamNum` (`self.GetPawnOwner`))) _revivecomponent)
    (else
      (return _returnvalue null))))

(fn `CheckToHeal`
  (params (Player :type "/HDCore/Core/BP_HDPlayerCharacterBase Object Reference"))
  (bind _returnvalue (`DFBasePlayerCharacter.GetCamera1P` Player))
  (bind _hitactor (`self.TraceForPawn` (`SceneComponent.K2_GetComponentLocation` _returnvalue) (`SceneComponent.GetForwardVector` _returnvalue) 50.0))
  (bind _isrevivable (`self.CheckIfRevivable` _hitactor))
  (set `self.CanHeal` _isrevivable)
  (return))

(fn `ClearTimer`
  (params (Handle :type "TimerHandle Structure (by ref)"))
  (if (`KismetSystemLibrary.K2_IsTimerActiveHandle` Handle)
    (`KismetSystemLibrary.K2_ClearAndInvalidateTimerHandle` Handle))
  (return))

(fn `PrintError`
  (params (Message :type String))
  (`KismetSystemLibrary.PrintString` (`KismetStringLibrary.Concat_StrStr` (`KismetStringLibrary.Concat_StrStr` (`KismetSystemLibrary.GetClassDisplayName` (`GameplayStatics.GetObjectClass` self)) ": ") Message) true true (struct :`R` 0.958533 :`B` 1.0 :`A` 1.0) 5.0))

(fn `TraceForPawn`
  (params (Origin :type "Vector Structure") (Direction :type "Vector Structure") (Offset :type "Float (double-precision)"))
  (returns (HitActor :type "Actor Object Reference"))
  (bind _outhit (`KismetSystemLibrary.LineTraceSingleForObjects` Origin (+ Origin (* Direction (+ (`self.DistanceToHeal`) Offset))) (`|MakeArray` "ObjectTypeQuery3" :!type "EObjectTypeQuery Enum") false (`|MakeArray` (`self.GetPawnOwner`) :!type "Actor Object Reference") "None" true (struct :`R` 1.0 :`A` 1.0) (struct :`G` 1.0 :`A` 1.0) 10.0))
  (return (`.HitActor` (`GameplayStatics.BreakHitResult` _outhit))))

(fn `UserConstructionScript`
  (`parent.UserConstructionScript`))