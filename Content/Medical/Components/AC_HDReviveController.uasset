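; Player controller component that lets medics revive wounded teammates and manages revive UI, including a wounded screen that hides the HUD.
; A looping timer shows registered wounded players' widgets by team and distance, with an input prompt in revive range.
; Reviving line-traces from the first-person camera, checks eligibility through interfaces and the target's revive component, then runs a gated hold-to-revive delay, cancelled on release.
; The revive executes directly with authority, otherwise via server RPC.
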(event `MedicTimer`
  ;[1 0.6023 0.9006] Revive Icon UI
  (`self.DisplayWoundedWidgets`))

(event `EnableMedicUI`
  (bind _medichandle (`self.MedicHandle`))
  ;[1 0.6023 0.9006] Revive Icon UI
  (`KismetSystemLibrary.PrintString` "MedicUIEnabled")
  (`self.HandleIsValid` _medichandle
    (:`True`
      (`KismetSystemLibrary.K2_UnPauseTimerHandle` _medichandle))
    (:`False`
      (bind _returnvalue (`KismetSystemLibrary.K2_SetTimerDelegate` (delegate `MedicTimer`) 0.3 true))
      (set `self.MedicHandle` _returnvalue))))

(event `self.ReceiveBeginPlay`
  (bind _controller (`self.Controller`))
  ;[0.4689 0.6298 1] BeginPlay
  (bind _asbp_hdplayer_controller_base (cast `/HDCore/Core/BP_HDPlayerControllerBase` (`self.GetOwner`))
    (:`then`
      (set `self.Controller` _asbp_hdplayer_controller_base)
      (`KismetSystemLibrary.PrintString` "ReviveControllerStarting" true true (struct :`R` 1.0 :`G` 0.970537 :`B` 0.992634 :`A` 1.0))
      (`/Engine/EditorBlueprintResources/StandardMacros.Can Execute Cosmetic Events`
        (:`True`
          (if (`Controller.IsLocalController` (`self.Controller`))
            (`self.LoadWoundedScreen`))
          (add `DFBasePlayerController.OnPossessPawn` _controller (`|CreateDelegate` :!event `OnPossess`))
          (add `DFBasePlayerController.OnUnpossessPawn` _controller (`|CreateDelegate` :!event `OnUnpossess`)))))
    (:`CastFailed`
      (`self.Deactivate`)
      (`self.PrintReviveControllerError` "ControllerCastFailed"))))

(event `DisableMedicUI`
  (bind _medichandle (`self.MedicHandle`))
  ;[1 0.6023 0.9006] Revive Icon UI
  (`KismetSystemLibrary.PrintString` "MedicUIDisabled")
  (`self.HandleIsValid` _medichandle
    (:`True`
      (`KismetSystemLibrary.K2_PauseTimerHandle` _medichandle))
    (:`False`
      _))
  (for _array_element (`self.WoundedPlayers`)
    (`SceneComponent.SetHiddenInGame` (`Actor.RootComponent` _array_element) true false)))

(event `OnUnpossess`
  (params (Pawn :type "Pawn Object Reference"))
  ;[1 0.6023 0.9006] Revive Icon UI
  (`self.DisableMedicUI`)
  (if (`Controller.IsLocalController` (`self.Controller`))
    (`self.WoundedScreenToggle` false)))

(event `RemoveWidget`
  (params (WoundedPlayer :type "/HDCore/Core/BP_HDPlayerCharacterBase Object Reference (by ref)"))
  ;[1 0.6023 0.9006] Revive Icon UI
  (`/Engine/EditorBlueprintResources/StandardMacros.IsValid` WoundedPlayer
    (:`Is Valid`
      (`KismetArrayLibrary.Array_RemoveItem` (`self.WoundedPlayers`) WoundedPlayer)
      (bind _revivewidget (message `/ConstructionPrototype/Medical/Interfaces/IF_Revivable.GetReviveWidget` WoundedPlayer))
      (`SceneComponent.SetHiddenInGame` _revivewidget true false))
    (:`Is Not Valid`
      (`self.PrintReviveControllerError` "RemoveInvalidWoundedPlayer"))))

(event `AddWidget`
  (params (WoundedPlayer :type "/HDCore/Core/BP_HDPlayerCharacterBase Object Reference (by ref)"))
  ;[1 0.6023 0.9006] Revive Icon UI
  (if (`KismetSystemLibrary.DoesImplementInterface` WoundedPlayer "/ConstructionPrototype/Medical/Interfaces/IF_Revivable.IF_Revivable_C")
    (`KismetArrayLibrary.Array_Add` (`self.WoundedPlayers`) WoundedPlayer)
    (else
      (`self.PrintReviveControllerError` "WoundedPlayer Needs To Have Revivable IF"))))

(event `RevivePlayer`
  (params (ReviveTarget :type "DFBaseCharacter Object Reference") (ReviveLocation :type "Vector Structure"))
  ;[0.4618 1 0.5753] Trace Actor then Initiate Revive
  ;;[1 0 0.7755] ReviveRPC
  (if (`DFBaseCharacter.IsAlive` ReviveTarget)
    (bind _revivecomponent (message `/ConstructionPrototype/Medical/Interfaces/IF_Revivable.GetReviveComponent` ReviveTarget))
    (if (`/ConstructionPrototype/Medical/Components/AC_HDReviveCharacter.IsRevivable` _revivecomponent (`DFBlueprintFunctions.GetTeamNum` (`self.GetOwner`)))
      (`/ConstructionPrototype/Medical/Components/AC_HDReviveCharacter.ReviveCharacterAtLocation` _revivecomponent ReviveLocation)
      (else
        (`self.PrintReviveControllerError` "ServerReviveFailed")))
    (else
      (`self.PrintReviveControllerError` "Dead"))))

(event `ServerRevivePlayer`
  (params (ReviveTarget :type "DFBaseCharacter Object Reference") (ReviveLocation :type "Vector Structure"))
  ;[0.4618 1 0.5753] Trace Actor then Initiate Revive
  ;;[1 0 0.7755] ReviveRPC
  (`self.RevivePlayer` ReviveTarget ReviveLocation))

(event `InitiateRevive`
  ;[0.4618 1 0.5753] Trace Actor then Initiate Revive
  (if (`/ConstructionPrototype/Medical/Components/AC_HDReviveCharacter.IsMedic` (`self.PlayerReviveComp`))
    (bind _out (`self.TraceForReviveTarget`)) ; Traces in Front of Revivng Pawn for Target Pawn
    (if (`KismetSystemLibrary.DoesImplementInterface` _out "/ConstructionPrototype/Medical/Interfaces/IF_Revivable.IF_Revivable_C")
      (bind _revivable_ (`self.CheckIfRevivable` _out)) ; Checks if Target Pawn shares team and is Wounded but still alive
      (if _revivable_
        (bind _asdfbase_character (cast `DFBaseCharacter` _out)
          (:`then`
            (bind _output_get (set `self.ReviveTarget` _asdfbase_character))
            (`self.CacheTargetReviveWidget` _output_get) ; Gets and stores Revive Widget from Revive Target
            (`self.HoldInputToRevive` (`self.ReviveHoldTime`) :!label _label ; Revive target player if Revivng player holds Use input
              (:`Exit`
                (if (`Actor.HasAuthority` (`self.GetOwner`))
                  (`self.RevivePlayer` (`self.ReviveTarget`) (`self.GetReviveLocation`)) ; Revives Player at clavicle bone location
                  (else
                    (`self.ServerRevivePlayer` (`self.ReviveTarget`) (`self.GetReviveLocation`)))))))
          (:`CastFailed`
            (`self.PrintReviveControllerError` "ReviveTargetIsNotPawn")))
        (else
          (`self.PrintReviveControllerError` "NotRevivable")))
      (else
        (`self.PrintReviveControllerError` "DoesntImplementRevivable")))
    (else
      (`self.PrintReviveControllerError` "NotMedic"))))

(event `OnPossess`
  (params (NewPawn :type "Pawn Object Reference"))
  ;[1 0.968 0.3904] Get Revive Component From Possessed Pawn
  (if (`KismetSystemLibrary.DoesImplementInterface` NewPawn "/ConstructionPrototype/Medical/Interfaces/IF_Revivable.IF_Revivable_C")
    (bind _revivecomponent (message `/ConstructionPrototype/Medical/Interfaces/IF_Revivable.GetReviveComponent` NewPawn))
    (`/Engine/EditorBlueprintResources/StandardMacros.IsValid` _revivecomponent
      (:`Is Valid`
        (set `self.PlayerReviveComp` _revivecomponent)
        (`KismetSystemLibrary.PrintString` "ComponentRetrieved"))
      (:`Is Not Valid`
        (`self.PrintReviveControllerError` "ComponentIsNotValid")))))

(event `ReleaseCancel`
  ;[0.4618 1 0.5753] Trace Actor then Initiate Revive
  (goto _label :!via `Release`))

(fn `CacheTargetReviveWidget`
  (params (Target :type "Object Object Reference"))
  (bind _revivewidget (message `/ConstructionPrototype/Medical/Interfaces/IF_Revivable.GetReviveWidget` Target))
  (bind _returnvalue (`WidgetComponent.GetUserWidgetObject` _revivewidget))
  (if (`KismetSystemLibrary.DoesImplementInterface` _returnvalue "/ConstructionPrototype/Medical/Interfaces/IF_ReviveUI.IF_ReviveUI_C")
    (set `self.TargetReviveWidget` _returnvalue)
    (else
      (`self.PrintReviveControllerError` "IF_ReviveUI not Implemented")))
  (return))

(fn `CheckIfRevivable`
  (params (ReviveTarget :type "Actor Object Reference"))
  (returns (`Revivable?` :type Boolean))
  (bind _revivecomponent (message `/ConstructionPrototype/Medical/Interfaces/IF_Revivable.GetReviveComponent` ReviveTarget))
  (return (`/ConstructionPrototype/Medical/Components/AC_HDReviveCharacter.IsRevivable` _revivecomponent (`DFBlueprintFunctions.GetTeamNum` (`self.GetOwner`)))))

(fn `DisplayWoundedWidgets`
  (locals (WidgetComponent :type "WidgetComponent Object Reference"))
  (for _array_element (`self.WoundedPlayers`)
    (bind _revivewidget (message `/ConstructionPrototype/Medical/Interfaces/IF_Revivable.GetReviveWidget` _array_element))
    (set `local.WidgetComponent` _revivewidget)
    (if (`self.CheckToDisplayMedicWidget` _array_element)
      (`SceneComponent.SetHiddenInGame` (`local.WidgetComponent`) true false)
      (else
        (`SceneComponent.SetHiddenInGame` (`local.WidgetComponent`) false false)
        (if (> (`self.GetDistanceToWoundedPawn` _array_element) (`self.DistanceToRevive`))
          (message `/ConstructionPrototype/Medical/Interfaces/IF_ReviveUI.ShowInput` (`WidgetComponent.GetUserWidgetObject` (`local.WidgetComponent`)) false)
          (else
            (message `/ConstructionPrototype/Medical/Interfaces/IF_ReviveUI.ShowInput` (`WidgetComponent.GetUserWidgetObject` (`local.WidgetComponent`)) true)))))))

(fn `GetDistanceToWoundedPawn`
  (params (Player :type "/HDCore/Core/BP_HDPlayerCharacterBase Object Reference"))
  (returns (Distance :type "Float (double-precision)"))
  (return (`KismetMathLibrary.Vector_Distance` (`Actor.K2_GetActorLocation` (`self.GetOwnerPawn`)) (`SceneComponent.GetSocketLocation` (`Character.Mesh` Player) "clavicle_r"))))

(fn `IsTeammate`
  (params (Object :type "Actor Object Reference"))
  (returns (ReturnValue :type Boolean))
  (return (== (`DFBlueprintFunctions.GetTeamNum` (`self.GetOwner`)) (`DFBlueprintFunctions.GetTeamNum` Object))))

(fn `LoadWoundedScreen`
  (`/Engine/EditorBlueprintResources/StandardMacros.IsValid` (`self.WoundedScreen`)
    (:`Is Not Valid`
      (bind _returnvalue (`|CreateWidget` "/ConstructionPrototype/Medical/UI/Revive/WBP_WoundedScreenRevive.WBP_WoundedScreenRevive_C" (`self.Controller`)))
      (set `self.WoundedScreen` _returnvalue))))

(fn `Show Medic UI`
  (params (Show :type Boolean))
  (if Show
    (`self.EnableMedicUI`)
    (else
      (`self.DisableMedicUI`))))

(fn `TraceForReviveTarget`
  (returns (Out :type "Actor Object Reference"))
  (bind _camera1p (`DFBasePlayerCharacter.Camera1P` (`self.GetOwnerPawn`)))
  (bind _returnvalue (`SceneComponent.K2_GetComponentLocation` _camera1p))
  (bind _outhit (`KismetSystemLibrary.LineTraceSingleForObjects` _returnvalue (+ _returnvalue (* (`SceneComponent.GetForwardVector` _camera1p) (`self.DistanceToRevive`))) (`self.TraceObjects`) false (`|MakeArray` (`self.GetOwnerPawn`) :!type "Actor Object Reference")))
  (return (`.HitActor` (`GameplayStatics.BreakHitResult` _outhit))))

(fn `WoundedScreenToggle`
  (params (Show :type Boolean))
  (locals (bWoundedScreenShown :type Boolean))
  (bind _woundedscreen (`self.WoundedScreen`))
  (bind _returnvalue (`Widget.IsInViewport` _woundedscreen))
  (`/Engine/EditorBlueprintResources/StandardMacros.IsValid` _woundedscreen
    (:`Is Valid`
      (if (`local.Show`)
        (if (not _returnvalue)
          (`UserWidget.AddToPlayerScreen` (`self.WoundedScreen`) 0)
          (bind _output_get (set `local.bWoundedScreenShown` (`local.Show`) :!label _label))
          (if _output_get
            (`/HDCore/Core/BP_HDPlayerControllerBase.HideHUD` (`self.Controller`))
            (else
              (`/HDCore/Core/BP_HDPlayerControllerBase.ShowHUD` (`self.Controller`)))))
        (elif _returnvalue
          (`Widget.RemoveFromParent` (`self.WoundedScreen`))
          (goto _label))))
    (:`Is Not Valid`
      (`self.PrintReviveControllerError` "WoundedWidgetNotValid"))))