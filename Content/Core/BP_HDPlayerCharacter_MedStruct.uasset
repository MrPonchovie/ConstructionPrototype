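; Player character Blueprint that adds medic and revive support through a revive component and a wounded-player widget.
; It initializes the component on possession, binds the widget to itself on BeginPlay, and rechecks medic status on the server when the loadout updates.
; The fire-press override runs a heal check before firing medical items, while preserving inventory-menu item selection except during a medical item's alt-fire.
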(event `self.ReceiveBeginPlay`
  (`parent.ReceiveBeginPlay`)
  (message `/ConstructionPrototype/Medical/Interfaces/IF_ReviveUI.SetWoundedOwner` (`WidgetComponent.GetUserWidgetObject` (`self.ReviveWidget`)) self))

(event `self.ReceivePossessed`
  (params (NewController :type "Controller Object Reference"))
  (`parent.ReceivePossessed` NewController)
  (`/ConstructionPrototype/Medical/Components/AC_HDReviveCharacter.Initialized` (`self.ReviveComponent`)) ; Wait for controller to be fully initialized and posses pawn before initializing component
)

(event `self.ReceiveCurrentLoadout`
  (`parent.ReceiveCurrentLoadout`)
  (`/Engine/EditorBlueprintResources/ActorMacros.Switch Has Authority`
    (:`Authority`
      (`/ConstructionPrototype/Medical/Components/AC_HDReviveCharacter.CheckIfMedic` (`self.ReviveComponent`)) ; If Kit Changed, Check if picked up kit is a medic kit
    )))

(event `self.OnPCFirePressed`
  (bind _asbp_hdmedical_base (cast `/ConstructionPrototype/Medical/Items/BP_HDMedicalBase` (`self.EquippedItem`))
    (:`then`
      (if (`/ConstructionPrototype/Medical/Items/BP_HDMedicalBase.IsAltFiring` _asbp_hdmedical_base)
        (`/ConstructionPrototype/Medical/Items/BP_HDMedicalBase.CheckToHeal` _asbp_hdmedical_base self)
        (`self.StartFire`)
        (elif (and (`self.bInventoryMenuShown`) (not (`self.bSelectingEquipmentBySlot`)))
          (`self.EquipSelectedItemFromInventory` true)
          (else
            (`/ConstructionPrototype/Medical/Items/BP_HDMedicalBase.CheckToHeal` _asbp_hdmedical_base self)
            (`self.StartFire`)))))
    (:`CastFailed`
      (if (and (`self.bInventoryMenuShown`) (not (`self.bSelectingEquipmentBySlot`)))
        (`self.EquipSelectedItemFromInventory` true)
        (else
          (`self.StartFire`))))))

(event `self.OnPCFireReleased`
  (`parent.OnPCFireReleased`))

(fn `GetReviveComponent`
  (returns (ReviveComponent :type "/ConstructionPrototype/Medical/Components/AC_HDReviveCharacter Object Reference"))
  (return (`self.ReviveComponent`)))

(fn `GetReviveWidget`
  (returns (ReviveWidget :type "WidgetComponent Object Reference"))
  (return (`self.ReviveWidget`)))

(fn `UserConstructionScript`
  (`parent.UserConstructionScript`))