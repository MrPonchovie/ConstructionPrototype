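; BP_HDPlayerCharacter_Med is a player character Blueprint that adds revive and medic-kit support on top of its parent character.
; It initializes its ReviveComponent on possession, after the parent logic, so that the controller is ready first.
; On current-loadout events, the authority has the component check whether the kit is a medic kit.
; Getter functions expose the revive component and revive widget.
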(event `self.ReceivePossessed`
  (params (NewController :type "Controller Object Reference"))
  (`parent.ReceivePossessed` NewController)
  (`/ConstructionPrototype/Core/Components/AC_HDReviveCharacter.Initialized` (`self.ReviveComponent`)) ; Wait for controller to be fully initialized and posses pawn before initializing component
)

(event `self.ReceiveCurrentLoadout`
  (`parent.ReceiveCurrentLoadout`)
  (`/Engine/EditorBlueprintResources/ActorMacros.Switch Has Authority`
    (:`Authority`
      (`/ConstructionPrototype/Core/Components/AC_HDReviveCharacter.CheckIfMedic` (`self.ReviveComponent`)) ; If Kit Changed, Check if picked up kit is a medic kit
    )))

(fn `GetReviveComponent`
  (returns (ReviveComponent :type "/ConstructionPrototype/Core/Components/AC_HDReviveCharacter Object Reference"))
  (return (`self.ReviveComponent`)))

(fn `GetReviveWidget`
  (returns (ReviveWidget :type "WidgetComponent Object Reference"))
  (return (`self.ReviveWidget`)))

(fn `UserConstructionScript`
  (`parent.UserConstructionScript`))