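; Base rangefinder weapon that reports distance and compass bearing to the aimed point.
; Equipping caches the player's HUD and shows a usage hint; construction registers its scope component as the current sight.
; Firing waits briefly, then line-traces forward from the first-person camera.
; A hit posts a HUD notification with distance in meters and bearing from look-at yaw between the item and impact point.
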(event `self.ReceiveOnEquip`
  (params (LastItem :type "DFBaseItem Object Reference"))
  (`parent.ReceiveOnEquip` LastItem)
  (bind _ashdplayer_controller (cast `HDPlayerController` (`/HDCore/Core/BPFL_HDCore.GetControllerFromPlayerState` (`Pawn.PlayerState` (`self.PawnOwner`))))
    (:`then`
      (`self.Get Valid Widget` _ashdplayer_controller)
      (`/HDCore/Core/BP_HDHUDBase.AddBasicNotification` (`self.Widget`) (make `/HDCore/UI/Notification/FUINotificationInfo` false 0 "NewEnumerator0" true "<Normal>Use \"Fire\" to get distance to point and compass bearing</>" "<Normal>{timer}</>")))
    (:`CastFailed`
      (`KismetSystemLibrary.PrintString` "NOT A REAL PLAYER" false false))))

(event `self.ReceiveFire`
  (`KismetSystemLibrary.Delay` 0.3)
  (bind (_outhit_distance _returnvalue _return_value_z__yaw_) (`self.Line Trace`))
  (if _returnvalue
    (`self.Display Distance and Bearing` _outhit_distance _return_value_z__yaw_)))

(event `Display Distance and Bearing`
  (params (Distance :type "Float (double-precision)") (Bearing :type "Float (double-precision)"))
  (`/HDCore/Core/BP_HDHUDBase.AddBasicNotification` (`self.Widget`) (make `/HDCore/UI/Notification/FUINotificationInfo` false 0 "NewEnumerator0" true (`KismetTextLibrary.Conv_StringToText` (`KismetStringLibrary.Concat_StrStr` "<Normal>Distance to point: " (`KismetStringLibrary.Conv_IntToString` (`KismetMathLibrary.Round` (/ Distance 100.0))) " meters. Compass bearing: " (`KismetTextLibrary.Conv_TextToString` (`KismetTextLibrary.Conv_DoubleToText` (`KismetMathLibrary.ClampAxis` Bearing) "ToZero" false true 1 324 0 0)) " degrees</>")) "<Normal>{timer}</>")))

(fn `Get Valid Widget`
  (params (NewParam :type "HDPlayerController Object Reference"))
  (bind _ashdhud (cast `HDHUD` (`PlayerController.GetHUD` NewParam))
    (:`then`
      (bind _asbp_hdhudbase (cast `/HDCore/Core/BP_HDHUDBase` _ashdhud)
        (:`then`
          (set `self.Widget` _asbp_hdhudbase))
        (:`CastFailed`
          (`KismetSystemLibrary.PrintString` "Failed BP Cast for HUD" false false (struct :`R` 1.0 :`B` 0.101476 :`A` 1.0)))))
    (:`CastFailed`
      (`KismetSystemLibrary.PrintString` "Failed C++ Cast for Hud" false false (struct :`R` 1.0 :`A` 1.0)))))

(fn `Line Trace`
  (returns (OutHit_Distance :type "Float (double-precision)") (ReturnValue :type Boolean) (`Return Value Z (Yaw)` :type "Float (double-precision)"))
  (`KismetSystemLibrary.PrintString` "Casted Ray" false false)
  (bind _asbp_hdplayer_character_base (cast `/HDCore/Core/BP_HDPlayerCharacterBase` (`self.GetPawnOwner`))
    (:`then`
      (bind _returnvalue (`DFBasePlayerCharacter.GetCamera1P` _asbp_hdplayer_character_base))
      (bind _returnvalue_2 (`SceneComponent.K2_GetComponentLocation` _returnvalue))
      (bind (_outhit _returnvalue_3) (`KismetSystemLibrary.LineTraceSingle` _returnvalue_2 (+ _returnvalue_2 (* (`SceneComponent.GetForwardVector` _returnvalue) (`self.TraceDistanceCM`))) "TraceTypeQuery3" false (`|MakeArray` (`self.GetPawnOwner`) self :!type "Actor Object Reference") "None" true (struct :`R` 1.0 :`A` 1.0) (struct :`G` 1.0 :`A` 1.0) 10.0))
      (bind (_returnvalue_roll _returnvalue_pitch _returnvalue_yaw) (`KismetMathLibrary.BreakRotator` (`KismetMathLibrary.FindLookAtRotation` (`self.K2_GetActorLocation`) (`.ImpactPoint` (`GameplayStatics.BreakHitResult` _outhit)))))
      (return (`.Distance` (`GameplayStatics.BreakHitResult` _outhit)) _returnvalue_3 _returnvalue_yaw))
    (:`CastFailed`
      (`KismetSystemLibrary.PrintString` "Missing Player Controller" false false))))

(fn `UserConstructionScript`
  (bind _bp_hdscopecomponentbase (`self.BP_HDScopeComponentBase`))
  (`parent.UserConstructionScript`)
  (set `self.Sights` (`|MakeArray` _bp_hdscopecomponentbase :!type "SceneComponent Object Reference"))
  (set `self.CurrentSight` _bp_hdscopecomponentbase))