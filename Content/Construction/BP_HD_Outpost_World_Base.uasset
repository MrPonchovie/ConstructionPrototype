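; Base team outpost that serves as a player spawn point and keeps nearby friendly buildables from decaying.
; Each Tick, sphere overlaps block spawning when enough enemies are inside the overrun radius, and claim same-team, unclaimed buildables within build range.
; Spawning also requires Built; spawn points get the actor transform added component-wise at BeginPlay and again in FindSpawnPointBP.
; Destruction starts decay on influenced buildables and releases their ownership.
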(event `self.ReceiveBeginPlay`
  (`parent.ReceiveBeginPlay`)
  (`self.SetUpSpawns`))

(event `self.Handle Destroy`
  (`self.SetActorTickEnabled` false)
  (for _array_element (`self.Influences`)
    (`self.Event Begin Decay` _array_element true)
    (set `/ConstructionPrototype/Construction/BP_HD_Buildable_World_Base.OwningOutpost` null _array_element))
  (`self.SetLifeSpan` 0.1))

(event `self.ReceiveTick`
  (params (DeltaSeconds :type "Float (single-precision)"))
  (`|ExecutionSequence`
    (:`then_0`
      (set `self.OwningOutpost` null)
      (bind _outactors (`KismetSystemLibrary.SphereOverlapActors` (`self.K2_GetActorLocation`) (`self.OverrunRadiusCM`) (`|MakeArray` "ObjectTypeQuery3" :!type "EObjectTypeQuery Enum") "/HDAssets/Core/BP_HDPlayerCharacter.BP_HDPlayerCharacter_C" (`|MakeArray` self :!type "Actor Object Reference")))
      (`self.EvalCanBeSpawnedAt` _outactors)
      (bind _outactors_2 (`KismetSystemLibrary.SphereOverlapActors` (`self.K2_GetActorLocation`) (`self.BuildRangeRadiusCM`) (`|MakeArray` "ObjectTypeQuery6" :!type "EObjectTypeQuery Enum") "/ConstructionPrototype/Construction/BP_HD_Buildable_World_Base.BP_HD_Buildable_World_Base_C" (`|MakeArray` self :!type "Actor Object Reference")))
      (for _array_element _outactors_2
        (bind _asbp_hd_buildable_world_base (cast `/ConstructionPrototype/Construction/BP_HD_Buildable_World_Base` _array_element))
        (`KismetArrayLibrary.Array_AddUnique` (`self.Influences`) _asbp_hd_buildable_world_base))
      (`self.CheckActorsInInfluence`)
      (for _array_element_2 (`self.Influences`)
        (set `/ConstructionPrototype/Construction/BP_HD_Buildable_World_Base.OwningOutpost` self _array_element_2)))
    (:`then_1`
      (`KismetSystemLibrary.Delay` 1.5)
      (`parent.ReceiveTick` DeltaSeconds))))

(fn `CanRestartPlayerFromSpawnPointBP`
  (params (SpawnPoint :type "SpawnPointDef Structure (by ref)") (Player :type "Controller Object Reference") (PlayerPawnClass :type "Pawn Class Reference"))
  (returns (ReturnValue :type Boolean))
  (return (and (`self.bBuilt`) (`self.CanBeSpawnedAt`))))

(fn `CanSpawnActorFromSpawnPointBP`
  (params (SpawnPoint :type "SpawnPointDef Structure (by ref)") (SpawnActorClass :type "Actor Class Reference"))
  (returns (ReturnValue :type Boolean))
  (return (and (`self.bBuilt`) (`self.CanBeSpawnedAt`))))

(fn `CheckActorsInInfluence`
  (locals (InvalidActors :type "Array of /ConstructionPrototype/Construction/BP_HD_Buildable_World_Base Object Reference"))
  (for _array_element (`self.Influences`)
    (`/Engine/EditorBlueprintResources/StandardMacros.IsValid` _array_element
      (:`Is Valid`
        (if (and (== (`self.OwningTeam`) (`/ConstructionPrototype/Construction/BP_HD_Buildable_World_Base.OwningTeam` _array_element)) (!= (`self.ActorHasTag` _array_element "HD_IgnoreRadio") true) (or (== (`/ConstructionPrototype/Construction/BP_HD_Buildable_World_Base.OwningOutpost` _array_element) self) (== (`/ConstructionPrototype/Construction/BP_HD_Buildable_World_Base.OwningOutpost` _array_element) null)))
          (set `/ConstructionPrototype/Construction/BP_HD_Buildable_World_Base.OwningOutpost` self _array_element)
          (`self.Event Halt Decay` _array_element)
          (else
            (`KismetArrayLibrary.Array_AddUnique` (`local.InvalidActors`) _array_element :!label _label))))
      (:`Is Not Valid`
        (goto _label))))
  (for _array_element_2 (`local.InvalidActors`)
    (`KismetArrayLibrary.Array_RemoveItem` (`self.Influences`) _array_element_2))
  (return))

(fn `EvalCanBeSpawnedAt`
  (params (Array :type "Array of Actor Object Reference"))
  (locals (Result :type Integer))
  (set `local.Result` 0)
  (for _array_element Array
    (bind _ashdplayer_character (cast `HDPlayerCharacter` _array_element))
    (if (not (`self.Is on Team` (`DFBaseCharacter.TeamNum` _ashdplayer_character)))
      (set `local.Result` (+ (`local.Result`) 1))))
  (set `self.CanBeSpawnedAt` (not (>= (`local.Result`) (`self.OverrunAmount`)))))

(fn `FindSpawnPointBP`
  (params (SpawnPointID :type Integer))
  (returns (FoundSpawnPoint :type "SpawnPointDef Structure") (ReturnValue :type Boolean))
  (bind (_returnvalue_roll _returnvalue_pitch _returnvalue_yaw) (`KismetMathLibrary.BreakRotator` (`self.K2_GetActorRotation`)))
  (bind _spawn_points (`self.Spawn Points`))
  (bind (_spawnid _spawntransform _spawncontextobject) (break `SpawnPointDef` (`|GetArrayItem` _spawn_points SpawnPointID)))
  (if (<= SpawnPointID (`KismetArrayLibrary.Array_Length` _spawn_points))
    (return (make `SpawnPointDef` _spawnid (`KismetMathLibrary.MakeTransform` (+ (.location _spawntransform) (`self.K2_GetActorLocation`)) (`KismetMathLibrary.MakeRotator` (+ (.roll (.rotation _spawntransform)) _returnvalue_roll) (+ (.pitch (.rotation _spawntransform)) _returnvalue_pitch) (+ (.yaw (.rotation _spawntransform)) _returnvalue_yaw)) (.scale _spawntransform)) _spawncontextobject) true)
    (else
      (return (struct) false))))

(fn `GetAllSpawnPointsBP`
  (returns (SpawnPoints :type "Array of SpawnPointDef Structure") (ReturnValue :type Integer))
  (bind _spawn_points (`self.Spawn Points`))
  (return _spawn_points (`KismetArrayLibrary.Array_Length` _spawn_points)))

(fn `GetSpawnPointCollisionHandlingOverrideBP`
  (params (SpawnPoint :type "SpawnPointDef Structure (by ref)"))
  (returns (OutSpawnCollisionMethod :type "ESpawnActorCollisionHandlingMethod Enum") (ReturnValue :type Boolean))
  (return "Undefined" true))

(fn `OnRep_CanBeSpawnedAt`)

(fn `SetUpSpawns`
  (bind (_returnvalue_roll _returnvalue_pitch _returnvalue_yaw) (`KismetMathLibrary.BreakRotator` (`self.K2_GetActorRotation`)))
  (for (_array_element _array_index) (`self.Spawn Points`)
    (`KismetArrayLibrary.Array_Set` (`self.Spawn Points`) _array_index (make `SpawnPointDef` (break `SpawnPointDef` _array_element) (`KismetMathLibrary.MakeTransform` (+ (.location (`.SpawnTransform` (break `SpawnPointDef` _array_element))) (`self.K2_GetActorLocation`)) (`KismetMathLibrary.MakeRotator` (+ (.roll (.rotation (`.SpawnTransform` (break `SpawnPointDef` _array_element)))) _returnvalue_roll) (+ (.pitch (.rotation (`.SpawnTransform` (break `SpawnPointDef` _array_element)))) _returnvalue_pitch) (+ (.yaw (.rotation (`.SpawnTransform` (break `SpawnPointDef` _array_element)))) _returnvalue_yaw)) (.scale (`.SpawnTransform` (break `SpawnPointDef` _array_element)))) (`.SpawnContextObject` (break `SpawnPointDef` _array_element))))))

(fn `UserConstructionScript`
  (`parent.UserConstructionScript`)
  (`SphereComponent.SetSphereRadius` (`self.BuildRangeSphere`) (`self.BuildRangeRadiusCM`) true)
  (`SphereComponent.SetSphereRadius` (`self.OverrunSphere`) (`self.OverrunRadiusCM`) true))