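; Base cooldown manager that tracks a countdown in whole-second steps and reports whether it has elapsed.
; SetCooldown resets SecondsRemaining to the Cooldown value and starts a looping one-second timer that calls TickCooldown by name to decrement it.
; CheckCooldown returns an elapsed flag and the remaining time.
; The timer is never cleared here, so the count keeps falling below zero.
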(fn `Check Cooldown`
  (returns (Elapsed :type Boolean) (`Time Remaining` :type Integer))
  (bind _secondsremaining (`self.SecondsRemaining`))
  (return (<= _secondsremaining 0) _secondsremaining))

(fn `Set Cooldown`
  (bind _returnvalue (`KismetSystemLibrary.K2_SetTimer` null "TickCooldown" 1.0 true))
  (set `self.CooldownTimer` _returnvalue)
  (set `self.SecondsRemaining` (`self.Cooldown`))
  (return))

(fn `TickCooldown`
  (set `self.SecondsRemaining` (- (`self.SecondsRemaining`) 1)))

(fn `UserConstructionScript`)