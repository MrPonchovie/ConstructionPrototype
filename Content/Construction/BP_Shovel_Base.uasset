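; Base shovel item that lets players build up or tear down tagged buildable world objects.
; Construct and Deconstruct set a server-side BuildMode, and replication of deconstruct mode triggers StartFire.
; On authority, Fire line-traces from the first-person camera, updates the buildable's health with the player's team, then multicasts tooltip progress and impact sound.
; Equipping creates the shovel UI and shows a keybind-aware hint; unequipping removes the UI.
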(event `Multicast Shovel`
  (params (NewParam2 :type String) (NewParam :type "Float (double-precision)") (NewParam3 :type "Vector Structure") (NewParam4 :type Boolean))
  (`/Engine/EditorBlueprintResources/StandardMacros.Can Execute Cosmetic Events`
    (:`True`
      (if NewParam4
        (`/ConstructionPrototype/Construction/WBP_Shovel_UI.Update Construction Tooltip` (`self.Widget`) NewParam2 NewParam)
        (`GameplayStatics.PlaySoundAtLocation` "/HDCore/Marketplace/BulletEffectsPack/BulletHitVFX_SFX/ESounds/Cue/SFX_Bullet_Impact_Sandbag.SFX_Bullet_Impact_Sandbag" NewParam3 (struct) 0.8 1.0 0.0 null null (`self.GetOwner`))))))

(event `Construct`
  (set `self.BuildMode` 0)
  (`self.Event Set Build Mode Server` 0))

(event `Deconstruct`
  (set `self.BuildMode` 1)
  (`self.Event Set Build Mode Server` 1))

(event `Event Set Build Mode Server`
  (params (`In Increment` :type Integer))
  (set `self.BuildMode` `In Increment`))

(event `Event Set Range Increment Server`
  (params (`In Increment` :type Integer))
  (set `self.Range Increment` `In Increment`))

(event `self.ReceiveFire`
  (bind _buildmode (`self.BuildMode`))
  (`/Engine/EditorBlueprintResources/ActorMacros.Switch Has Authority`
    (:`Authority`
      (`KismetSystemLibrary.PrintString` (`KismetStringLibrary.Conv_IntToString` _buildmode))
      (switch `int` _buildmode
        (:`0`
          (bind (_uiname _returnvalue _outputpin _returnvalue1) (`self.Linetrace_0`))
          (`self.Multicast Shovel` _uiname _returnvalue _outputpin _returnvalue1))
        (:`1`
          (bind (_uiname_2 _returnvalue_2 _outputpin_2 _returnvalue1_2) (`self.Linetrace_1`))
          (`self.Multicast Shovel` _uiname_2 _returnvalue_2 _outputpin_2 _returnvalue1_2))))))

(event `self.ReceiveOnUnEquip`
  (params (bPlayAnimAndWait :type Boolean) (bLeavingPawnInventory :type Boolean))
  (`parent.ReceiveOnUnEquip` bPlayAnimAndWait bLeavingPawnInventory)
  (`/Engine/EditorBlueprintResources/StandardMacros.Can Execute Cosmetic Events`
    (:`True`
      (`Widget.RemoveFromParent` (`self.Widget`)))))

(event `self.ReceiveOnEquip`
  (params (LastItem :type "DFBaseItem Object Reference"))
  (bind _ownerc (`/HDCore/Core/BPFL_HDCore.GetControllerFromPlayerState` (`Pawn.PlayerState` (`self.PawnOwner`))))
  (`parent.ReceiveOnEquip` LastItem)
  (`/Engine/EditorBlueprintResources/StandardMacros.Can Execute Cosmetic Events`
    (:`True`
      (bind _foundwidgets (`WidgetBlueprintLibrary.GetAllWidgetsOfClass` "/ConstructionPrototype/Construction/WBP_Shovel_UI.WBP_Shovel_UI_C"))
      (for _array_element _foundwidgets
        (if (== (`Widget.GetOwningPlayer` _array_element) _ownerc)
          (`Widget.RemoveFromParent` _array_element)))
      (bind _asbp_hdplayer_controller (cast `/HDAssets/Core/BP_HDPlayerController` _ownerc)
        (:`then`
          (`self.Get Valid Notification Widget` _asbp_hdplayer_controller)
          (`self.Show Initial Notification`)
          (bind _returnvalue (`|CreateWidget` "/ConstructionPrototype/Construction/WBP_Shovel_UI.WBP_Shovel_UI_C" _asbp_hdplayer_controller))
          (bind _output_get (set `self.Widget` _returnvalue))
          (`UserWidget.AddToPlayerScreen` _output_get 1))
        (:`CastFailed`
          (`KismetSystemLibrary.PrintString` "NOT A REAL PLAYER"))))))

(event `Show Initial Notification`
  (bind (_output_actionname _output_bshift _output_bctrl _output_balt _output_bcmd _output_key) (break `InputActionKeyMapping` (`|GetArrayItem` (`InputSettings.GetActionMappingByName` (`InputSettings.GetInputSettings`) "AimToggle"))))
  (bind (_output_actionname_2 _output_bshift_2 _output_bctrl_2 _output_balt_2 _output_bcmd_2 _output_key_2) (break `InputActionKeyMapping` (`|GetArrayItem` (`InputSettings.GetActionMappingByName` (`InputSettings.GetInputSettings`) "Fire"))))
  (bind (_output_actionname_3 _output_bshift_3 _output_bctrl_3 _output_balt_3 _output_bcmd_3 _output_key_3) (break `InputActionKeyMapping` (`|GetArrayItem` (`InputSettings.GetActionMappingByName` (`InputSettings.GetInputSettings`) "Aim"))))
  (bind _returnvalue (`KismetTextLibrary.Conv_TextToString` (`KismetInputLibrary.Key_GetDisplayName` _output_key_2)))
  (bind _returnvalue_2 (`KismetTextLibrary.Conv_TextToString` (`KismetInputLibrary.Key_GetDisplayName` _output_key)))
  (bind _returnvalue_3 (`KismetTextLibrary.Conv_TextToString` (`KismetInputLibrary.Key_GetDisplayName` _output_key_3)))
  (bind _returnvalue_4 (`KismetStringLibrary.EqualEqual_StrStr` _returnvalue_2))
  (if (`KismetStringLibrary.EqualEqual_StrStr` _returnvalue_3)
    (if _returnvalue_4
      (`/HDCore/Core/BP_HDHUDBase.AddBasicNotification` (`self.Notification Widget`) (make `/HDCore/UI/Notification/FUINotificationInfo` false 0 "NewEnumerator0" true "<Normal>Please bind the \"Fire\" and \"AimToggle\" or \"Aim\" keybinds to use this item properly</>" "" 10.0))
      (else
        ;[1 1 1] AimToggle Keybind Active
        (`/HDCore/Core/BP_HDHUDBase.AddBasicNotification` (`self.Notification Widget`) (make `/HDCore/UI/Notification/FUINotificationInfo` false 0 "NewEnumerator0" true (`KismetTextLibrary.Conv_StringToText` (`KismetStringLibrary.Concat_StrStr` "<Normal>Use \"" _returnvalue "\" to build and \"" _returnvalue_2 "\" to destroy</>")) "" 10.0))))
    (elif _returnvalue_4
      ;[1 1 1] AimToggle Keybind Active
      (`/HDCore/Core/BP_HDHUDBase.AddBasicNotification` (`self.Notification Widget`) (make `/HDCore/UI/Notification/FUINotificationInfo` false 0 "NewEnumerator0" true (`KismetTextLibrary.Conv_StringToText` (`KismetStringLibrary.Concat_StrStr` "<Normal>Use \"" _returnvalue "\" to build and \"" _returnvalue_3 "\" to destroy</>")) "" 10.0))
      (else
        ;[1 1 1] Both Keybinds Active
        (`/HDCore/Core/BP_HDHUDBase.AddBasicNotification` (`self.Notification Widget`) (make `/HDCore/UI/Notification/FUINotificationInfo` false 0 "NewEnumerator0" true (`KismetTextLibrary.Conv_StringToText` (`KismetStringLibrary.Concat_StrStr` "<Normal>Use \"" _returnvalue "\" to build and \"" _returnvalue_2 "\" or \"" _returnvalue_3 "\" to destroy</>")) "" 10.0))))))

(fn `Convert Degree Inc to Range Inc`
  (params (`Degree Increment` :type Integer))
  (returns (`Range Increment` :type Integer))
  (switch `int` `Degree Increment`
    (:`Default`
      _)
    (:`1`
      (bind _output_get (set `self.Range Increment` 1))
      (return _output_get))
    (:`2`
      _)
    (:`3`
      _)
    (:`4`
      _)
    (:`5`
      (bind _output_get_2 (set `self.Range Increment` 2))
      (return _output_get_2))
    (:`6`
      _)
    (:`7`
      _)
    (:`8`
      _)
    (:`9`
      _)
    (:`10`
      (bind _output_get_3 (set `self.Range Increment` 4))
      (return _output_get_3)))
  (`KismetSystemLibrary.PrintString` "Invalid Range Increment!" true true (struct :`R` 1.0 :`A` 1.0)))

(fn `Generic Notification`
  (params (`Info Text` :type Text))
  (`/HDCore/Core/BP_HDHUDBase.AddBasicNotification` (`self.Notification Widget`) (make `/HDCore/UI/Notification/FUINotificationInfo` false 0 "NewEnumerator0" true `Info Text` "")))

(fn `Get Valid Notification Widget`
  (params (Target :type "PlayerController Object Reference"))
  (bind _ashdhud (cast `HDHUD` (`PlayerController.GetHUD` Target))
    (:`then`
      (bind _asbp_hdhudbase (cast `/HDCore/Core/BP_HDHUDBase` _ashdhud)
        (:`then`
          (set `self.Notification Widget` _asbp_hdhudbase))
        (:`CastFailed`
          (`KismetSystemLibrary.PrintString` "Failed BP Cast for HUD" true true (struct :`R` 1.0 :`B` 0.101476 :`A` 1.0)))))
    (:`CastFailed`
      (`KismetSystemLibrary.PrintString` "Failed C++ Cast for Hud" true true (struct :`R` 1.0 :`A` 1.0)))))

(fn `Linetrace_0`
  (returns (UIName :type String) (ReturnValue :type "Float (double-precision)") (OutputPin :type "Vector Structure") (ReturnValue1 :type Boolean))
  (bind _returnvalue (`DFBasePlayerCharacter.GetCamera1P` (`self.Player`)))
  (bind _returnvalue_2 (`SceneComponent.K2_GetComponentLocation` _returnvalue))
  (`/Engine/EditorBlueprintResources/StandardMacros.IsValid` (`self.Player`) :!label _label
    (:`Is Valid`
      (bind (_outhit _returnvalue_3) (`KismetSystemLibrary.LineTraceSingle` _returnvalue_2 (+ _returnvalue_2 (* (`SceneComponent.GetForwardVector` _returnvalue) (`self.Trace DistanceCM`))) "TraceTypeQuery3" false (`|MakeArray` (`self.GetPawnOwner`) self :!type "Actor Object Reference") "ForDuration"))
      (if _returnvalue_3
        (bind (_bblockinghit _binitialoverlap _time _distance _location _impactpoint _normal _impactnormal _physmat _hitactor) (`GameplayStatics.BreakHitResult` _outhit))
        (if (`self.ActorHasTag` _hitactor "Buildable_Object")
          (bind _asbp_hd_buildable_world_base (cast `/ConstructionPrototype/Construction/BP_HD_Buildable_World_Base` _hitactor)
            (:`then`
              (bind _new_health (`/ConstructionPrototype/Construction/BP_HD_Buildable_World_Base.FuncUpdateHealth` _asbp_hd_buildable_world_base 34.0 0 (`DFBlueprintFunctions.GetTeamNum` (`self.Player`))))
              (return (`/ConstructionPrototype/Construction/BP_HD_Buildable_World_Base.UIName` _asbp_hd_buildable_world_base) (/ _new_health (`/ConstructionPrototype/Construction/BP_HD_Buildable_World_Base.MaximumHealth` _asbp_hd_buildable_world_base)) _location _returnvalue_3))
            (:`CastFailed`
              (`DFBlueprintFunctions.PrintTextToLog` "Cast to HD_Buildable_Object failed despite filters" "Error" true)))
          (else
            (`KismetSystemLibrary.PrintString` "Object doesn't have Buildable tag, ignoring." true true (struct :`R` 1.0 :`G` 0.879168 :`A` 1.0))))
        (else
          (`DFBlueprintFunctions.PrintTextToLog` "Caught nothing in shovel line trace. (NOTE: This is NOT an error)" "Warning"))))
    (:`Is Not Valid`
      (bind _ashdplayer_character (cast `HDPlayerCharacter` (`self.GetPawnOwner`))
        (:`then`
          (set `self.Player` _ashdplayer_character)
          (goto _label))
        (:`CastFailed`
          (`DFBlueprintFunctions.PrintTextToLog` "Failed to cast to C++ Controller" "Error" true)))))
  (return "" 0.0 (0.0 0.0 0.0) false))

(fn `Linetrace_1`
  (returns (UIName :type String) (ReturnValue :type "Float (double-precision)") (OutputPin :type "Vector Structure") (ReturnValue1 :type Boolean))
  (bind _returnvalue (`DFBasePlayerCharacter.GetCamera1P` (`self.Player`)))
  (bind _returnvalue_2 (`SceneComponent.K2_GetComponentLocation` _returnvalue))
  (`/Engine/EditorBlueprintResources/StandardMacros.IsValid` (`self.Player`) :!label _label
    (:`Is Valid`
      (bind (_outhit _returnvalue_3) (`KismetSystemLibrary.LineTraceSingle` _returnvalue_2 (+ _returnvalue_2 (* (`SceneComponent.GetForwardVector` _returnvalue) (`self.Trace DistanceCM`))) "TraceTypeQuery3" false (`|MakeArray` (`self.GetPawnOwner`) self :!type "Actor Object Reference") "ForDuration"))
      (if _returnvalue_3
        (bind (_bblockinghit _binitialoverlap _time _distance _location _impactpoint _normal _impactnormal _physmat _hitactor) (`GameplayStatics.BreakHitResult` _outhit))
        (if (`self.ActorHasTag` _hitactor "Buildable_Object")
          (bind _asbp_hd_buildable_world_base (cast `/ConstructionPrototype/Construction/BP_HD_Buildable_World_Base` _hitactor)
            (:`then`
              (bind _new_health (`/ConstructionPrototype/Construction/BP_HD_Buildable_World_Base.FuncUpdateHealth` _asbp_hd_buildable_world_base 34.0 1 (`DFBlueprintFunctions.GetTeamNum` (`self.Player`))))
              (return (`/ConstructionPrototype/Construction/BP_HD_Buildable_World_Base.UIName` _asbp_hd_buildable_world_base) (/ _new_health (`/ConstructionPrototype/Construction/BP_HD_Buildable_World_Base.MaximumHealth` _asbp_hd_buildable_world_base)) _location _returnvalue_3))
            (:`CastFailed`
              (`DFBlueprintFunctions.PrintTextToLog` "Cast to HD_Buildable_Object failed despite filters" "Error" true)))
          (else
            (`KismetSystemLibrary.PrintString` "Object doesn't have Buildable tag, ignoring." true true (struct :`R` 1.0 :`G` 0.879168 :`A` 1.0))))
        (else
          (`DFBlueprintFunctions.PrintTextToLog` "Caught nothing in shovel line trace. (NOTE: This is NOT an error)" "Warning"))))
    (:`Is Not Valid`
      (bind _ashdplayer_character (cast `HDPlayerCharacter` (`self.GetPawnOwner`))
        (:`then`
          (set `self.Player` _ashdplayer_character)
          (goto _label))
        (:`CastFailed`
          (`DFBlueprintFunctions.PrintTextToLog` "Failed to cast to C++ Controller" "Error" true))))))

(fn `OnRep_BuildMode`
  (bind _buildmode (`self.BuildMode`))
  (`KismetSystemLibrary.PrintString` (`KismetStringLibrary.Conv_IntToString` _buildmode))
  (switch `int` _buildmode
    (:`1`
      (`self.StartFire`))))

(fn `Read Component Tags`
  (returns (`Out Increment` :type Integer))
  (bind _returnvalue (`KismetStringLibrary.Conv_StringToInt` (`KismetStringLibrary.Conv_NameToString` (`|GetArrayItem` (`ActorComponent.ComponentTags` (`self.CurrentSight`))))))
  (bind _output_get (set `self.BuildMode` _returnvalue))
  (`KismetSystemLibrary.PrintString` (`KismetStringLibrary.Conv_IntToString` _returnvalue) true true (struct :`R` 1.0 :`B` 0.915568 :`A` 1.0))
  (return _output_get))

(fn `UserConstructionScript`
  (bind _building (`self.Building`))
  (`parent.UserConstructionScript`)
  (set `self.Sights` (`|MakeArray` _building (`self.UnBuild`)))
  (set `self.CurrentSight` _building))