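; BP_Buildable_Ghost_Preview is the ghost actor that previews a buildable's placement during construction.
; Its Update event moves and rotates the actor, applies the given mesh, and swaps every material slot to green or red dev glass based on validity.
; A near-zero location acts as a sentinel that gives the ghost a very short lifespan, removing it instead of updating it.
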(event `Update`
  (params (Mesh :type "StaticMesh Object Reference") (Valid :type Boolean) (Location :type "Vector Structure") (Rotation :type "Rotator Structure"))
  (if (== Location (0.0 0.0 0.0))
    (`self.SetLifeSpan` 0.1)
    (else
      (`self.K2_SetActorRotation` Rotation)
      (`self.K2_SetActorLocation` Location)
      (`StaticMeshComponent.SetStaticMesh` (`self.StaticMesh`) Mesh)
      (if Valid
        (for (_ _array_index) (`MeshComponent.GetMaterials` (`self.StaticMesh`))
          (`PrimitiveComponent.SetMaterial` (`self.StaticMesh`) _array_index "/HDCore/Marketplace/BlockingStarterPack/Materials/Glass/MI_DevGlassGreen.MI_DevGlassGreen"))
        (else
          (for (_ _array_index_2) (`MeshComponent.GetMaterials` (`self.StaticMesh`))
            (`PrimitiveComponent.SetMaterial` (`self.StaticMesh`) _array_index_2 "/HDCore/Marketplace/BlockingStarterPack/Materials/Glass/MI_DevGlassRed.MI_DevGlassRed")))))))

(fn `UserConstructionScript`)