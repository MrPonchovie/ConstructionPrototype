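; Base squad rally point placed in the world, serving as a team spawn location.
; On ownership setup it offsets its spawn points by the actor transform and expires any other rally of the same squad.
; An enemy player inside the overrun radius, at setup or on overlap, destroys it and notifies the owning player's HUD.
; Spawn-point queries always permit spawning; lookup by ID adds the actor offset again.
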(event `self.Event SetupOwnership`
  (params (`Owning Team` :type Byte) (`Owning Squad` :type "HDSquadState Object Reference"))
  (`parent.Event SetupOwnership` `Owning Team` `Owning Squad`)
  (`self.SetUpSpawnPoints`)
  (bind _outactors (`GameplayStatics.GetAllActorsOfClass` "BP_HD_Rally_World_Base_C"))
  (if (> (`KismetArrayLibrary.Array_Length` _outactors) 0)
    (for _array_element _outactors
      (if (== _array_element self)
        _
        (elif (== (`/ConstructionPrototype/Construction/BP_HD_Buildable_World_Base.OwningSquad` _array_element) (`self.OwningSquad`))
          (`self.SetLifeSpan` _array_element 0.1))))
    (bind _outactors_2 (`KismetSystemLibrary.SphereOverlapActors` (`self.K2_GetActorLocation`) (`self.OverrunRadiusCM`) (`|MakeArray` "ObjectTypeQuery3" :!type "EObjectTypeQuery Enum") "/HDAssets/Core/BP_HDPlayerCharacter.BP_HDPlayerCharacter_C" (`|MakeArray` self :!type "Actor Object Reference")))
    (for _array_element_2 _outactors_2
      (bind _ashdplayer_character (cast `HDPlayerCharacter` _array_element_2))
      (if (not (`self.Is on Team` (`DFBaseCharacter.TeamNum` _ashdplayer_character)))
        (`self.Handle Destroy`)))))

(event `self.OverrunSphere.OnComponentBeginOverlap`
  (params (OverlappedComponent :type "PrimitiveComponent Object Reference") (OtherActor :type "Actor Object Reference") (OtherComp :type "PrimitiveComponent Object Reference") (OtherBodyIndex :type Integer) (bFromSweep :type Boolean) (SweepResult :type "HitResult Structure (by ref)"))
  ;[1 1 1] Rally burning
  (bind _ashdplayer_character (cast `HDPlayerCharacter` OtherActor))
  (if (not (`self.Is on Team` (`DFBaseCharacter.TeamNum` _ashdplayer_character)))
    (`self.Handle Destroy`)))

(event `self.Handle Destroy`
  (`parent.Handle Destroy`)
  (bind _ashdplayer_controller (cast `HDPlayerController` (`self.GetOwner`)))
  (bind _ashdhud (cast `HDHUD` (`PlayerController.GetHUD` _ashdplayer_controller))
    (:`then`
      (bind _asbp_hdhudbase (cast `/HDCore/Core/BP_HDHUDBase` _ashdhud)
        (:`then`
          (set `self.Notification Widget` _asbp_hdhudbase)
          (`/HDCore/Core/BP_HDHUDBase.AddBasicNotification` (`self.Notification Widget`) (make `/HDCore/UI/Notification/FUINotificationInfo` false 0 "NewEnumerator0" true "<Normal>Your squad's rally point has been destroyed!</>" "<Normal>{timer}</>")))
        (:`CastFailed`
          (`KismetSystemLibrary.PrintString` "Failed BP Cast for HUD" true true (struct :`R` 1.0 :`B` 0.101476 :`A` 1.0)))))
    (:`CastFailed`
      (`KismetSystemLibrary.PrintString` "Failed C++ Cast for Hud" true true (struct :`R` 1.0 :`A` 1.0)))))

(fn `CanRestartPlayerFromSpawnPointBP`
  (params (SpawnPoint :type "SpawnPointDef Structure (by ref)") (Player :type "Controller Object Reference") (PlayerPawnClass :type "Pawn Class Reference"))
  (returns (ReturnValue :type Boolean))
  (return true))

(fn `CanSpawnActorFromSpawnPointBP`
  (params (SpawnPoint :type "SpawnPointDef Structure (by ref)") (SpawnActorClass :type "Actor Class Reference"))
  (returns (ReturnValue :type Boolean))
  (return true))

(fn `FindSpawnPointBP`
  (params (SpawnPointID :type Integer))
  (returns (FoundSpawnPoint :type "SpawnPointDef Structure") (ReturnValue :type Boolean))
  (bind (_returnvalue_roll _returnvalue_pitch _returnvalue_yaw) (`KismetMathLibrary.BreakRotator` (`self.K2_GetActorRotation`)))
  (bind _spawn_points (`self.Spawn Points`))
  (bind (_spawnid _spawntransform _spawncontextobject) (break `SpawnPointDef` (`|GetArrayItem` _spawn_points SpawnPointID)))
  (if (<= SpawnPointID (`KismetArrayLibrary.Array_Length` _spawn_points))
    (return (make `SpawnPointDef` _spawnid (`KismetMathLibrary.MakeTransform` (+ (.location _spawntransform) (`self.K2_GetActorLocation`)) (`KismetMathLibrary.MakeRotator` (+ (.roll (.rotation _spawntransform)) _returnvalue_roll) (+ (.pitch (.rotation _spawntransform)) _returnvalue_pitch) (+ (.yaw (.rotation _spawntransform)) _returnvalue_yaw)) (.scale _spawntransform)) _spawncontextobject) true)
    (else
      (return (struct) false))))

(fn `GetAllSpawnPointsBP`
  (returns (SpawnPoints :type "Array of SpawnPointDef Structure") (ReturnValue :type Integer))
  (bind _spawn_points (`self.Spawn Points`))
  (return _spawn_points (`KismetArrayLibrary.Array_Length` _spawn_points)))

(fn `GetSpawnPointCollisionHandlingOverrideBP`
  (params (SpawnPoint :type "SpawnPointDef Structure (by ref)"))
  (returns (OutSpawnCollisionMethod :type "ESpawnActorCollisionHandlingMethod Enum") (ReturnValue :type Boolean))
  (return "Undefined" true))

(fn `SetUpSpawnPoints`
  (bind (_returnvalue_roll _returnvalue_pitch _returnvalue_yaw) (`KismetMathLibrary.BreakRotator` (`self.K2_GetActorRotation`)))
  (for (_array_element _array_index) (`self.Spawn Points`)
    (`KismetArrayLibrary.Array_Set` (`self.Spawn Points`) _array_index (make `SpawnPointDef` (break `SpawnPointDef` _array_element) (`KismetMathLibrary.MakeTransform` (+ (.location (`.SpawnTransform` (break `SpawnPointDef` _array_element))) (`self.K2_GetActorLocation`)) (`KismetMathLibrary.MakeRotator` (+ (.roll (.rotation (`.SpawnTransform` (break `SpawnPointDef` _array_element)))) _returnvalue_roll) (+ (.pitch (.rotation (`.SpawnTransform` (break `SpawnPointDef` _array_element)))) _returnvalue_pitch) (+ (.yaw (.rotation (`.SpawnTransform` (break `SpawnPointDef` _array_element)))) _returnvalue_yaw)) (.scale (`.SpawnTransform` (break `SpawnPointDef` _array_element)))) (`.SpawnContextObject` (break `SpawnPointDef` _array_element))))))

(fn `UserConstructionScript`
  (`parent.UserConstructionScript`)
  (`SphereComponent.SetSphereRadius` (`self.OverrunSphere`) (`self.OverrunRadiusCM`) true))